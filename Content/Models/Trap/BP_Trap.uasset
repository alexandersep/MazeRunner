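; BP_Trap is a lethal trap that ends the game when BP_TopDownCharacter overlaps its box.
; The overlap plays the trap animation and sounds, ragdolls and immobilizes the character, and spawns blood.
; It starts streaming GameOver, then after a short delay opens that level, clearing victory and key count on BP_GameInstance.
; Initialize snaps the trap onto its owner at a reduced fraction of the owner's scale.
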(event OnComponentBeginOverlap(Box)
  (params (OverlappedComponent :type Primitive%20Component%20Object%20Reference) (OtherActor :type Actor%20Object%20Reference) (OtherComp :type Primitive%20Component%20Object%20Reference) (OtherBodyIndex :type Integer) (bFromSweep :type Boolean) (SweepResult :type Hit%20Result%20Structure%20%28by%20ref%29))
  (bind _asbp_top_down_character (Utilities|Casting|CastToBP_TopDownCharacter OtherActor))
  (Audio|PlaySoundatLocation "/Game/Models/Trap/SFX_Stab.SFX_Stab" (Transformation|GetActorLocation _asbp_top_down_character) "0, 0, 0" 1.0 1.0 0.2 0 0 0 0)
  (Components|Animation|PlayAnimation (Variables|Default|GetTrap) "/Game/Models/Trap/trap_Anim.trap_Anim" false)
  (Audio|PlaySound2D "/Game/Models/Blood/game-over-arcade-sound.game-over-arcade-sound" 1.0 1.0 0.0 0 0)
  (Default|Ragdoll _asbp_top_down_character)
  (Pawn|Components|CharacterMovement|DisableMovement (Variables|/Script/Engine.Character|GetCharacterMovement _asbp_top_down_character))
  (Niagara|SpawnSystematLocation "/Game/Models/Blood/NS_Blood.NS_Blood" (Transformation|GetActorLocation _asbp_top_down_character))
  (Game|LoadStreamLevel(byName) "GameOver" true)
  (Utilities|FlowControl|Delay 1.3)
  (bind _asbp_game_instance (Utilities|Casting|CastToBP_GameInstance (Game|GetGameInstance)))
  (Variables|/Game/Blueprints/BP_GameInstance.BP_GameInstance_C|Setvictory _asbp_game_instance false)
  (Game|OpenLevel(byName) "GameOver")
  (Variables|/Game/Blueprints/BP_GameInstance.BP_GameInstance_C|SetamountOfKeys _asbp_game_instance 0))

(event EventBeginPlay)

(event Collision|EventActorBeginOverlap
  (params (OtherActor :type Actor%20Object%20Reference)))

(event EventTick
  (params (DeltaSeconds :type Float%20%28single-precision%29)))

(fn ConstructionScript)

(fn Initialize
  (bind _returnvalue (Components|GetOwner))
  (Utilities|IsValid _returnvalue
    (:Is%20Valid
      (Transformation|AttachActorToActor _returnvalue "None" "SnapToTarget" "SnapToTarget" "SnapToTarget" true)
      (Transformation|SetActorScale3D (* (Transformation|GetActorScale3D _returnvalue) "0.300000,0.300000,0.300000")))))