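; BP_Tile is a tile actor that takes its place in a grid relative to the actor that owns it.
; Initialize, given a Scale, snaps the tile onto its owner, then offsets it by Column along X and Row along Y.
; The grid spacing comes from the Tile component's bounds at that scale, applied to the actor last.
; Without a valid owner it does nothing.
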(event EventBeginPlay)

(event Collision|EventActorBeginOverlap
  (params (OtherActor :type Actor%20Object%20Reference)))

(event EventTick
  (params (DeltaSeconds :type Float%20%28single-precision%29)))

(fn ConstructionScript)

(fn Initialize
  (params (Scale :type Vector))
  (bind _returnvalue (Components|GetOwner))
  (bind _tile (Variables|Default|GetTile))
  (bind _boxextent (Collision|GetComponentBounds _tile))
  (bind _returnvalue_2 (* _boxextent "2.000000,2.000000,1.000000"))
  (bind _returnvalue_3 (* _returnvalue_2 Scale))
  (bind (_x _y) (Math|Vector|BreakVector _returnvalue_3))
  (Utilities|IsValid _returnvalue
    (:Is%20Valid
      (Transformation|AttachActorToActor _returnvalue "None" "SnapToTarget" "SnapToTarget" "SnapToTarget" true)
      (Transformation|SetActorRelativeLocation (Math|Vector|MakeVector (* (* _x (Variables|Default|GetColumn)) 1.0) (* (* _y (Variables|Default|GetRow)) 1.0) 0.0))
      (Transformation|SetActorScale3D Scale))))