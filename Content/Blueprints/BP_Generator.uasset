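; BP_Generator builds a tile-based maze actor with walls, corners, keys and traps.
; GenerateMaze takes wall, corner, content and solution data from a temporary MazeGenerator, then recursively destroys attached actors before spawning a Rows x Columns tile grid.
; Each tile's 4-bit wall and corner masks select a piece class and yaw, while its content code spawns items.
; Start and end positions are stored, but RenderStartAndEnd is an empty stub.
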(event EventBeginPlay)

(event Collision|EventActorBeginOverlap
  (params (OtherActor :type Actor%20Object%20Reference)))

(event EventTick
  (params (DeltaSeconds :type Float%20%28single-precision%29)))

(fn ConstructionScript)

(fn GenerateMaze
  (CallFunction|SetupMazeData)
  (CallFunction|ClearMaze)
  (for _index (range 0 (- (Variables|Default|GetRows) 1))
    (for _index_2 (range 0 (- (Variables|Default|GetColumns) 1))
      (bind _returnvalue (Game|SpawnActorfromClass "/Game/Blueprints/BP_Tile.BP_Tile_C" (Math|Transform|MakeTransform (Transformation|GetActorLocation) (Transformation|GetActorRotation)) "AlwaysSpawn" "MultiplyWithRoot" self _index _index_2 0 0))
      (Default|Initialize _returnvalue (Math|Vector|MakeVector 5.0 5.0 2.0))
      (Utilities|FlowControl|Sequence
        (:then_0
          (CallFunction|RenderTileWalls _returnvalue (+ (* _index (Variables|Default|GetColumns)) _index_2)))
        (:then_1
          (CallFunction|RenderTileCorners (+ (* _index (Variables|Default|GetColumns)) _index_2) _returnvalue))
        (:then_2
          (CallFunction|RenderItems (+ (* _index (Variables|Default|GetColumns)) _index_2) _returnvalue))))
    (CallFunction|RenderStartandEnd)))

(fn DeleteChildren
  (params (Children :type Array%20of%20Actor%20Object%20References))
  (if (> (Utilities|Array|Length Children) 0)
    (for _array_element Children
      (CallFunction|DeleteChildren (Actor|GetAttachedActors _array_element false false))
      (Actor|DestroyActor _array_element))))

(fn SetupMazeData
  (bind _returnvalue (Game|SpawnActorfromClass "/Script/MazeRunner.MazeGenerator" (Transformation|GetActorTransform self) "AlwaysSpawn" "MultiplyWithRoot" 0 0))
  (bind _returnvalue_2 (Class|MazeGenerator|GenerateMaze _returnvalue (Variables|Default|GetRows) (Variables|Default|GetColumns)))
  (Utilities|FlowControl|Sequence
    (:then_0
      (Variables|Default|SetcornersGrid (Variables|/Script/MazeRunner.MazeGenerator|GetcornersGrid _returnvalue)))
    (:then_1
      (Variables|Default|SetwallsGrid _returnvalue_2))
    (:then_2
      (Variables|Default|Setsolution (Variables|/Script/MazeRunner.MazeGenerator|Getsolution _returnvalue)))
    (:then_3
      (Variables|Default|SetstartPos (Utilities|Array|Get(acopy) (Variables|/Script/MazeRunner.MazeGenerator|Getsolution _returnvalue))))
    (:then_4
      (Variables|Default|SetendPos (Utilities|Array|Get(acopy) (Variables|/Script/MazeRunner.MazeGenerator|Getsolution _returnvalue) (- (Utilities|Array|Length (Variables|/Script/MazeRunner.MazeGenerator|Getsolution _returnvalue)) 1))))
    (:then_5
      (Variables|Default|SettileContentsGrid (Variables|/Script/MazeRunner.MazeGenerator|GettileContentsGrid _returnvalue)))
    (:then_6
      (Actor|DestroyActor _returnvalue))))

(fn ClearMaze
  (CallFunction|DeleteChildren (Actor|GetAttachedActors self true false)))

(fn RenderTileWalls
  (params (Tile :type BP%20Tile%20Object%20Reference) (Tile%20Index :type Integer))
  (bind _returnvalue (Transformation|GetActorRotation Tile))
  (bind (_roll _pitch _yaw) (Math|Rotator|BreakRotator _returnvalue))
  (bind _returnvalue_2 (+ _yaw -9e+01))
  (bind _returnvalue_3 (+ _yaw 0.0))
  (bind _returnvalue_4 (+ _yaw 9e+01))
  (bind _returnvalue_5 (+ _yaw 1.8e+02))
  (bind _returnvalue_6 (Math|Rotator|MakeRotator 0.0 0.0 _returnvalue_2))
  (bind _returnvalue_7 (Math|Rotator|MakeRotator _roll _pitch _returnvalue_3))
  (bind _returnvalue_8 (Math|Rotator|MakeRotator 0.0 0.0 _returnvalue_4))
  (bind _returnvalue_9 (Math|Rotator|MakeRotator 0.0 0.0 _returnvalue_5))
  (bind _returnvalue_10 (Math|Transform|MakeTransform "0, 0, 0" _returnvalue_6))
  (bind _returnvalue_11 (Math|Transform|MakeTransform "0, 0, 0" _returnvalue_7))
  (bind _returnvalue_12 (Math|Transform|MakeTransform "0, 0, 0" _returnvalue_8))
  (bind _returnvalue_13 (Math|Transform|MakeTransform "0, 0, 0" _returnvalue_9))
  (switch int (Utilities|Array|Get(acopy) (Variables|Default|GetwallsGrid) Tile%20Index)
    (:0
      (return 0))
    (:1
      ;[1 1 1] Wall (1 bit)
      (bind _returnvalue_14 (Game|SpawnActorfromClass "/Game/Blueprints/BP_Tile_Wall.BP_Tile_Wall_C" _returnvalue_11 "AlwaysSpawn" "MultiplyWithRoot" Tile 0))
      (Default|Init _returnvalue_14)
      (return _returnvalue_14))
    (:2
      (bind _returnvalue_15 (Game|SpawnActorfromClass "/Game/Blueprints/BP_Tile_Wall.BP_Tile_Wall_C" _returnvalue_13 "AlwaysSpawn" "MultiplyWithRoot" Tile 0))
      (Default|Init _returnvalue_15)
      (return _returnvalue_15))
    (:3
      ;[1 1 1] Sides (2 bits)
      (bind _returnvalue_16 (Game|SpawnActorfromClass "/Game/Blueprints/BP_Tile_Wall_Sides.BP_Tile_Wall_Sides_C" _returnvalue_11 "AlwaysSpawn" "MultiplyWithRoot" Tile 0))
      (Default|Init _returnvalue_16))
    (:4
      (bind _returnvalue_17 (Game|SpawnActorfromClass "/Game/Blueprints/BP_Tile_Wall.BP_Tile_Wall_C" _returnvalue_12 "AlwaysSpawn" "MultiplyWithRoot" Tile 0))
      (Default|Init _returnvalue_17)
      (return _returnvalue_17))
    (:5
      ;[1 1 1] Corner (2 bits)
      (bind _returnvalue_18 (Game|SpawnActorfromClass "/Game/Blueprints/BP_Tile_Wall_Corner.BP_Tile_Wall_Corner_C" _returnvalue_11 "AlwaysSpawn" "MultiplyWithRoot" Tile 0))
      (Default|Init _returnvalue_18)
      (return _returnvalue_18))
    (:6
      (bind _returnvalue_19 (Game|SpawnActorfromClass "/Game/Blueprints/BP_Tile_Wall_Corner.BP_Tile_Wall_Corner_C" _returnvalue_12 "AlwaysSpawn" "MultiplyWithRoot" Tile 0))
      (Default|Init _returnvalue_19)
      (return _returnvalue_19))
    (:7
      ;[1 1 1] End (3 bits)
      (bind _returnvalue_20 (Game|SpawnActorfromClass "/Game/Blueprints/BP_Tile_Wall_End.BP_Tile_Wall_End_C" _returnvalue_12 "AlwaysSpawn" "MultiplyWithRoot" Tile 0))
      (Default|Init _returnvalue_20))
    (:8
      (bind _returnvalue_21 (Game|SpawnActorfromClass "/Game/Blueprints/BP_Tile_Wall.BP_Tile_Wall_C" _returnvalue_10 "AlwaysSpawn" "MultiplyWithRoot" Tile 0))
      (Default|Init _returnvalue_21)
      (return _returnvalue_21))
    (:9
      (bind _returnvalue_22 (Game|SpawnActorfromClass "/Game/Blueprints/BP_Tile_Wall_Corner.BP_Tile_Wall_Corner_C" _returnvalue_10 "AlwaysSpawn" "MultiplyWithRoot" Tile 0))
      (Default|Init _returnvalue_22)
      (return _returnvalue_22))
    (:10
      (bind _returnvalue_23 (Game|SpawnActorfromClass "/Game/Blueprints/BP_Tile_Wall_Corner.BP_Tile_Wall_Corner_C" _returnvalue_13 "AlwaysSpawn" "MultiplyWithRoot" Tile 0))
      (Default|Init _returnvalue_23)
      (return _returnvalue_23))
    (:11
      (bind _returnvalue_24 (Game|SpawnActorfromClass "/Game/Blueprints/BP_Tile_Wall_End.BP_Tile_Wall_End_C" _returnvalue_10 "AlwaysSpawn" "MultiplyWithRoot" Tile 0))
      (Default|Init _returnvalue_24))
    (:12
      (bind _returnvalue_25 (Game|SpawnActorfromClass "/Game/Blueprints/BP_Tile_Wall_Sides.BP_Tile_Wall_Sides_C" _returnvalue_12 "AlwaysSpawn" "MultiplyWithRoot" Tile 0))
      (Default|Init _returnvalue_25))
    (:13
      (bind _returnvalue_26 (Game|SpawnActorfromClass "/Game/Blueprints/BP_Tile_Wall_End.BP_Tile_Wall_End_C" _returnvalue_11 "AlwaysSpawn" "MultiplyWithRoot" Tile 0))
      (Default|Init _returnvalue_26))
    (:14
      (bind _returnvalue_27 (Game|SpawnActorfromClass "/Game/Blueprints/BP_Tile_Wall_End.BP_Tile_Wall_End_C" _returnvalue_13 "AlwaysSpawn" "MultiplyWithRoot" Tile 0))
      (Default|Init _returnvalue_27))
    (:15
      ;[1 1 1] Full (4 bits)
      (bind _returnvalue_28 (Game|SpawnActorfromClass "/Game/Blueprints/BP_Tile_Wall_Full.BP_Tile_Wall_Full_C" _returnvalue_11 "AlwaysSpawn" "MultiplyWithRoot" Tile 0))
      (Default|Init _returnvalue_28)
      (return _returnvalue_28))))

(fn RenderTileCorners
  (params (Corners%20Grid%20Index :type Integer) (Tile :type Actor%20Object%20Reference))
  (bind _returnvalue (Transformation|GetActorRotation Tile))
  (bind (_roll _pitch _yaw) (Math|Rotator|BreakRotator _returnvalue))
  (bind _returnvalue_2 (+ _yaw -9e+01))
  (bind _returnvalue_3 (+ _yaw 0.0))
  (bind _returnvalue_4 (+ _yaw 9e+01))
  (bind _returnvalue_5 (+ _yaw 1.8e+02))
  (bind _returnvalue_6 (Math|Rotator|MakeRotator 0.0 0.0 _returnvalue_2))
  (bind _returnvalue_7 (Math|Rotator|MakeRotator _roll _pitch _returnvalue_3))
  (bind _returnvalue_8 (Math|Rotator|MakeRotator 0.0 0.0 _returnvalue_4))
  (bind _returnvalue_9 (Math|Rotator|MakeRotator 0.0 0.0 _returnvalue_5))
  (bind _returnvalue_10 (Math|Transform|MakeTransform "0, 0, 0" _returnvalue_6))
  (bind _returnvalue_11 (Math|Transform|MakeTransform "0, 0, 0" _returnvalue_7))
  (bind _returnvalue_12 (Math|Transform|MakeTransform "0, 0, 0" _returnvalue_8))
  (bind _returnvalue_13 (Math|Transform|MakeTransform "0, 0, 0" _returnvalue_9))
  (switch int (Utilities|Array|Get(acopy) (Variables|Default|GetcornersGrid) Corners%20Grid%20Index)
    (:1
      ;[1 1 1] Wall (1 bit)
      (bind _returnvalue_14 (Game|SpawnActorfromClass "/Game/Blueprints/BP_Tile_Corner.BP_Tile_Corner_C" _returnvalue_11 "AlwaysSpawn" "MultiplyWithRoot" Tile 0))
      (Default|Init _returnvalue_14)
      (return _returnvalue_14))
    (:2
      (bind _returnvalue_15 (Game|SpawnActorfromClass "/Game/Blueprints/BP_Tile_Corner.BP_Tile_Corner_C" _returnvalue_12 "AlwaysSpawn" "MultiplyWithRoot" Tile 0))
      (Default|Init _returnvalue_15)
      (return _returnvalue_15))
    (:3
      ;[1 1 1] Corner (2 bits)
      (bind _returnvalue_16 (Game|SpawnActorfromClass "/Game/Blueprints/BP_Tile_Two_Corners.BP_Tile_Two_Corners_C" _returnvalue_11 "AlwaysSpawn" "MultiplyWithRoot" Tile 0))
      (Default|Init _returnvalue_16)
      (return _returnvalue_16))
    (:4
      (bind _returnvalue_17 (Game|SpawnActorfromClass "/Game/Blueprints/BP_Tile_Corner.BP_Tile_Corner_C" _returnvalue_10 "AlwaysSpawn" "MultiplyWithRoot" Tile 0))
      (Default|Init _returnvalue_17)
      (return _returnvalue_17))
    (:5
      (bind _returnvalue_18 (Game|SpawnActorfromClass "/Game/Blueprints/BP_Tile_Two_Corners.BP_Tile_Two_Corners_C" _returnvalue_10 "AlwaysSpawn" "MultiplyWithRoot" Tile 0))
      (Default|Init _returnvalue_18)
      (return _returnvalue_18))
    (:6
      ;[1 1 1] Sides (2 bits)
      (bind _returnvalue_19 (Game|SpawnActorfromClass "/Game/Blueprints/BP_Tile_Opposite_Corners.BP_Tile_Opposite_Corners_C" _returnvalue_12 "AlwaysSpawn" "MultiplyWithRoot" Tile 0))
      (Default|Init _returnvalue_19)
      (return _returnvalue_19))
    (:7
      ;[1 1 1] End (3 bits)
      (bind _returnvalue_20 (Game|SpawnActorfromClass "/Game/Blueprints/BP_Tile_Three_Corners.BP_Tile_Three_Corners_C" _returnvalue_11 "AlwaysSpawn" "MultiplyWithRoot" Tile 0))
      (Default|Init _returnvalue_20)
      (return _returnvalue_20))
    (:8
      (bind _returnvalue_21 (Game|SpawnActorfromClass "/Game/Blueprints/BP_Tile_Corner.BP_Tile_Corner_C" _returnvalue_13 "AlwaysSpawn" "MultiplyWithRoot" Tile 0))
      (Default|Init _returnvalue_21)
      (return _returnvalue_21))
    (:9
      (bind _returnvalue_22 (Game|SpawnActorfromClass "/Game/Blueprints/BP_Tile_Opposite_Corners.BP_Tile_Opposite_Corners_C" _returnvalue_11 "AlwaysSpawn" "MultiplyWithRoot" Tile 0))
      (Default|Init _returnvalue_22)
      (return _returnvalue_22))
    (:10
      (bind _returnvalue_23 (Game|SpawnActorfromClass "/Game/Blueprints/BP_Tile_Two_Corners.BP_Tile_Two_Corners_C" _returnvalue_12 "AlwaysSpawn" "MultiplyWithRoot" Tile 0))
      (Default|Init _returnvalue_23)
      (return _returnvalue_23))
    (:11
      (bind _returnvalue_24 (Game|SpawnActorfromClass "/Game/Blueprints/BP_Tile_Three_Corners.BP_Tile_Three_Corners_C" _returnvalue_12 "AlwaysSpawn" "MultiplyWithRoot" Tile 0))
      (Default|Init _returnvalue_24)
      (return _returnvalue_24))
    (:12
      (bind _returnvalue_25 (Game|SpawnActorfromClass "/Game/Blueprints/BP_Tile_Two_Corners.BP_Tile_Two_Corners_C" _returnvalue_13 "AlwaysSpawn" "MultiplyWithRoot" Tile 0))
      (Default|Init _returnvalue_25)
      (return _returnvalue_25))
    (:13
      (bind _returnvalue_26 (Game|SpawnActorfromClass "/Game/Blueprints/BP_Tile_Three_Corners.BP_Tile_Three_Corners_C" _returnvalue_10 "AlwaysSpawn" "MultiplyWithRoot" Tile 0))
      (Default|Init _returnvalue_26)
      (return _returnvalue_26))
    (:14
      (bind _returnvalue_27 (Game|SpawnActorfromClass "/Game/Blueprints/BP_Tile_Three_Corners.BP_Tile_Three_Corners_C" _returnvalue_13 "AlwaysSpawn" "MultiplyWithRoot" Tile 0))
      (Default|Init _returnvalue_27)
      (return _returnvalue_27))
    (:15
      ;[1 1 1] Full (4 bits)
      (bind _returnvalue_28 (Game|SpawnActorfromClass "/Game/Blueprints/BP_Tile_FourCorners.BP_Tile_FourCorners_C" _returnvalue_11 "AlwaysSpawn" "MultiplyWithRoot" Tile 0))
      (Default|Init _returnvalue_28)
      (return _returnvalue_28))))

(fn RenderStartandEnd)

(fn RenderItems
  (params (index :type Integer) (tile :type BP%20Tile%20Object%20Reference))
  (bind _returnvalue (Math|Transform|MakeTransform "0, 0, 0"))
  (switch int (Utilities|Array|Get(acopy) (Variables|Default|GettileContentsGrid) index)
    (:1
      (bind _returnvalue_2 (Game|SpawnActorfromClass "/Game/Models/Key/KeyActor.KeyActor_C" _returnvalue "AlwaysSpawn" "MultiplyWithRoot" tile 0))
      (Default|Initialize _returnvalue_2 "1.000000,1.000000,2.000000")
      (return _returnvalue_2 0))
    (:4
      (bind _returnvalue_3 (Game|SpawnActorfromClass "/Game/Models/Trap/BP_Trap.BP_Trap_C" _returnvalue "AlwaysSpawn" "MultiplyWithRoot" tile 0))
      (Default|Initialize _returnvalue_3)
      (return 0 _returnvalue_3))))