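; Zombie AI enemy that roams to random reachable points nearby and chases pawns it sees through PawnSensing.
; Roaming is a self-restarting AIMoveTo loop that sets a running animation on each arrival.
; A sighting re-arms CanAttack and moves to the pawn, playing a jump attack after a delay on arrival, with no damage logic.
; A retriggerable delay restarts roaming once sightings stop for a moment.
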(event OnSeePawn(PawnSensing)
  (params (Pawn :type Pawn%20Object%20Reference))
  (Utilities|FlowControl|Sequence
    (:then_0
      (Variables|Default|SetCanAttack true)
      (AI|AIMoveTo self "0, 0, 0" Pawn 5e+01 false
        (:OnSuccess
          (if (Variables|Default|GetCanAttack)
            (Variables|Default|SetCanAttack false)
            (Utilities|FlowControl|Delay 3.0)
            (Components|Animation|PlayAnimation (Variables|Character|GetMesh) "/Game/AI/Jump_Attack.Jump_Attack" false)
            (else
              (Components|Animation|SetAnimation (Variables|Character|GetMesh) "/Game/AI/BlendSpace.BlendSpace"))))))
    (:then_1
      (Utilities|FlowControl|RetriggerableDelay 1.0)
      (CallFunction|RandomRoam))))

(event Custom|Random%20Roam
  (AI|AIMoveTo self (.RandomLocation (AI|Navigation|GetRandomReachablePointinRadius (Transformation|GetActorLocation) 2.5e+03 0 0)) 0 5e+01 false
    (:OnSuccess
      (Components|Animation|SetAnimation (Variables|Character|GetMesh) "/Game/AI/Zombie_Running_Anim.Zombie_Running_Anim")
      (CallFunction|RandomRoam))))

(event EventBeginPlay
  (CallFunction|RandomRoam))

(event Collision|EventActorBeginOverlap
  (params (OtherActor :type Actor%20Object%20Reference)))

(fn ConstructionScript)